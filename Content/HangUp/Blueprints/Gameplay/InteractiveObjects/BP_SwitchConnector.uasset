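; BP_SwitchConnector is an interactive connector that reports being inserted or removed to the level's switchboard.
; On BeginPlay it caches the first BP_SwitchBoard found through GetAllActorsOfClass, without checking that one exists.
; Its INSERT and Remove events pass the connector itself to the board's Connected and Disconnected calls, leaving any connection logic to the board.
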(event `self.ReceiveBeginPlay`
  (bind _outactors (`GameplayStatics.GetAllActorsOfClass` "/Game/HangUp/Blueprints/Gameplay/InteractiveObjects/BP_SwitchBoard.BP_SwitchBoard_C"))
  (set `self.BoardRef` (`|GetArrayItem` _outactors)))

(event `self.iNSERT`
  (`/Game/HangUp/Blueprints/Gameplay/InteractiveObjects/BP_SwitchBoard.Connected` (`self.BoardRef`) self))

(event `self.Remove`
  (`/Game/HangUp/Blueprints/Gameplay/InteractiveObjects/BP_SwitchBoard.Disconnected` (`self.BoardRef`) self))

(fn `UserConstructionScript`)