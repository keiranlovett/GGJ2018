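; TriggerConditionButtons is a trigger condition that is met when a target interactable, by its name a button, is pressed.
; On BeginPlay it binds to the target actor's Pressed event, whose handler sets IsSuccess to true and prints a debug string.
; Nothing here resets the flag.
; Nodes for calling TriggerCondition and restarting a SequencePlayer are present but unconnected.
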(event `self.ReceiveBeginPlay`
  (add `/Game/HangUp/Blueprints/Gameplay/InteractiveObjects/BP_InteractiveButton.Pressed` (`self.interactableTargetActor`) (delegate `Toggled_Event_0`)))

(event `Toggled_Event_0`
  (set `self.isSuccess` true)
  (`KismetSystemLibrary.PrintString` "puahsh evevnt"))