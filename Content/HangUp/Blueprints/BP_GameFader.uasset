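; BP_GameFader is an actor that drives a screen fade, apparently a whitewipe, through the MPC_Whitewipe material parameter collection.
; Every tick it teleports its root to the player camera's location.
; FadeOut plays a timeline or reverses it from the end depending on its FadeIn flag, writing the track to the Fade parameter and stopping at zero or below.
; Clear resets Fade to zero.
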(event `self.ReceiveTick`
  (params (DeltaSeconds :type "Float (single-precision)"))
  (`SceneComponent.K2_SetWorldLocationAndRotation` :`self` (`self.DefaultSceneRoot`) :`NewLocation` (`PlayerCameraManager.GetCameraLocation` (`GameplayStatics.GetPlayerCameraManager` 0)) :`bTeleport` true))

(event `FadeOut`
  (params (fadeIn :type Boolean))
  (if fadeIn
    ;[1 1 1] Fade in
    (bind (_direction _newtrack_0) (`Timeline|Timeline_0` :`NewTime` 3.0 :!label _label)
      (:`Update`
        (`KismetMaterialLibrary.SetScalarParameterValue` "/Game/HangUp/Geometry/Materials/MPC_Whitewipe.MPC_Whitewipe" "Fade" _newtrack_0)
        (if (<= _newtrack_0 0.0)
          (goto _label :!via `Stop`))))
    (else
      (goto _label :!via `ReverseFromEnd`))))

(event `Clear`
  (`KismetMaterialLibrary.SetScalarParameterValue` "/Game/HangUp/Geometry/Materials/MPC_Whitewipe.MPC_Whitewipe" "Fade"))

(fn `UserConstructionScript`)