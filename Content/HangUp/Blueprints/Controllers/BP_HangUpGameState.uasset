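; Game state for HangUp that tracks stage progression and player failure, announcing both through event dispatchers.
; Triggers register in a map of fired flags, and only those matching the current stage can be triggered or detriggered.
; Triggering scans that stage's flags to decide whether to advance through three stages to GameOver.
; A separate failure counter signals game failure at its maximum and can be reset only below it.
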(fn `DetriggerStageEvent`
  (params (StageTrigger :type "/Game/HangUp/Blueprints/EnumStruct/StageTrigger Structure"))
  (locals (currentStageTrigger :type "/Game/HangUp/Blueprints/EnumStruct/StageTrigger Structure"))
  (bind _currentstagetrigger (`local.currentStageTrigger`))
  (bind _stagetriggers (`self.StageTriggers`))
  ;[1 1 1] Determine if the trigger belongs to the currentStage
  (bind _output_get (set `local.currentStageTrigger` StageTrigger))
  (if (`|EnumEquality` (`.GameStage_4_89D143F247BF1D649460F6AA79CB2324` (break `/Game/HangUp/Blueprints/EnumStruct/StageTrigger` _output_get)) (`self.CurrentStage`))
    ;[1 1 1] Update stage triggers
    (bind _returnvalue (`BlueprintMapLibrary.Map_Remove` _stagetriggers _currentstagetrigger))
    (if _returnvalue
      (`BlueprintMapLibrary.Map_Add` _stagetriggers _currentstagetrigger)
      (else
        (`KismetSystemLibrary.PrintString` "There's no such Trigger")))))

(fn `IncrementFailureLevel`
  (bind _result (`/Engine/EditorBlueprintResources/StandardMacros.IncrementInt` (`self.CurrentFailureLevel`))
    (:`  `
      (`|ExecutionSequence`
        (:`then_0`
          (if (<= _result (`self.MaxFailureLevel`))
            (`self.FailureLevelIncremented` _result)))
        (:`then_1`
          (if (== _result (`self.MaxFailureLevel`))
            (`self.GameFailed`)))))))

(fn `RegisterStageTrigger`
  (params (NewTrigger :type "/Game/HangUp/Blueprints/EnumStruct/StageTrigger Structure"))
  (`BlueprintMapLibrary.Map_Add` (`self.StageTriggers`) NewTrigger))

(fn `ResetFailureLevel`
  (if (< (`self.CurrentFailureLevel`) (`self.MaxFailureLevel`))
    (set `self.CurrentFailureLevel` 0)))

(fn `TriggerStageEvent`
  (params (StageTrigger :type "/Game/HangUp/Blueprints/EnumStruct/StageTrigger Structure"))
  (returns (Success :type Boolean))
  (locals (currentStageOver :type Boolean :default true) (bCurrentStageTriggerMap :type "Array of Boolean") (currentStageTrigger :type "/Game/HangUp/Blueprints/EnumStruct/StageTrigger Structure") (bResult :type Boolean))
  (bind _bcurrentstagetriggermap (`local.bCurrentStageTriggerMap`))
  (bind _currentstagetrigger (`local.currentStageTrigger`))
  (bind _stagetriggers (`self.StageTriggers`))
  ;[1 1 1] Determine if the trigger belongs to the currentStage
  (bind _output_get (set `local.currentStageTrigger` StageTrigger))
  (if (`|EnumEquality` (`.GameStage_4_89D143F247BF1D649460F6AA79CB2324` (break `/Game/HangUp/Blueprints/EnumStruct/StageTrigger` _output_get)) (`self.CurrentStage`))
    (`|ExecutionSequence`
      (:`then_0`
        ;[1 1 1] Update stage triggers
        (bind _returnvalue (`BlueprintMapLibrary.Map_Remove` _stagetriggers _currentstagetrigger))
        (if _returnvalue
          (`BlueprintMapLibrary.Map_Add` _stagetriggers _currentstagetrigger true)
          ;[1 1 1] Populate a trigger Map for the current Stage
          (bind _keys (`BlueprintMapLibrary.Map_Keys` (`self.StageTriggers`)))
          (for _array_element _keys
            (if (`|EnumEquality` (`self.CurrentStage`) (`.GameStage_4_89D143F247BF1D649460F6AA79CB2324` (break `/Game/HangUp/Blueprints/EnumStruct/StageTrigger` _array_element)))
              (`KismetArrayLibrary.Array_Add` (`local.bCurrentStageTriggerMap`) (`BlueprintMapLibrary.Map_Find` (`self.StageTriggers`) _array_element))))
          (else
            (`KismetSystemLibrary.PrintString` "There's no such Trigger"))))
      (:`then_1`
        ;[1 1 1] Check to see if we need to pass to the next stage
        (if (!= (`KismetArrayLibrary.Array_Length` _bcurrentstagetriggermap) 0)
          (for _array_element_2 _bcurrentstagetriggermap
            (if (not _array_element_2)
              (set `local.currentStageOver` false)
              (break)))
          (else
            (set `local.currentStageOver` false))))
      (:`then_2`
        ;[1 1 1] Execute Stage Over if needed
        (if (`local.currentStageOver`)
          (`self.IncrementStage`)))
      (:`then_3`
        (set `local.bResult` true))
      (:`then_4`
        (return (`local.bResult`))))
    (else
      (set `local.bResult` false)
      (return (`local.bResult`)))))

(fn `UserConstructionScript`)