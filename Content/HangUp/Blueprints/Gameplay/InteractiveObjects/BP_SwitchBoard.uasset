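; BP_SwitchBoard is the switchboard puzzle actor that tracks whether the correct switch connectors are plugged in across three game stages.
; On BeginPlay it gathers all connectors, registers stage triggers with BP_HangUpGameState and randomly picks the required connections.
; Connected and Disconnected count correct plugs, registering the current stage's trigger when complete or detriggering on a correct unplug.
; Stage completion reshuffles the pins, resets the failure level and prints a placeholder phone-call message.
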(event `self.ReceiveBeginPlay`
  (bind _outactors (`GameplayStatics.GetAllActorsOfClass` "/Game/HangUp/Blueprints/Gameplay/InteractiveObjects/BP_SwitchConnector.BP_SwitchConnector_C"))
  (set `self.AllSwitchConnectors` _outactors)
  (bind _asbp_hang_up_game_state (cast `/Game/HangUp/Blueprints/Controllers/BP_HangUpGameState` (`GameplayStatics.GetGameState`)))
  (set `self.GameStateRef` _asbp_hang_up_game_state)
  (`self.InitializeBoard`)
  (`self.ShufflePins`)
  (add `/Game/HangUp/Blueprints/Controllers/BP_HangUpGameState.StageOver` (`self.GameStateRef`) (delegate `OnStageOver`)))

(event `OnStageOver`
  (params (StageID :type "/Game/HangUp/Blueprints/EnumStruct/GameStage Enum" :default "NewEnumerator1"))
  (`|ExecutionSequence`
    (:`then_0`
      (`self.ShufflePins`)
      (`/Game/HangUp/Blueprints/Controllers/BP_HangUpGameState.ResetFailureLevel` (`self.GameStateRef`)))
    (:`then_1`
      (switch `/Game/HangUp/Blueprints/EnumStruct/GameStage` StageID
        (:`NewEnumerator1`
          (`KismetSystemLibrary.PrintString` "Phone call 1 is here"))
        (:`NewEnumerator2`
          (`KismetSystemLibrary.PrintString` "Phone call 2 is here"))
        (:`NewEnumerator3`
          (`KismetSystemLibrary.PrintString` "Phone call 3 is here"))))))

(fn `Connected`
  (params (Connector :type "/Game/HangUp/Blueprints/Gameplay/InteractiveObjects/BP_SwitchConnector Object Reference"))
  (returns (Match :type Boolean))
  (locals (bResult :type Boolean))
  (bind _correct (`self.IsConnectionCorrect` Connector))
  (bind _output_get (set `local.bResult` _correct))
  (if _output_get
    (bind _result (`/Engine/EditorBlueprintResources/StandardMacros.IncrementInt` (`self.CurrentConnectionCount`))
      (:`  `
        (if (== _result (`self.TotalConnectionNeeded`))
          (`/Game/HangUp/Blueprints/Controllers/BP_HangUpGameState.RegisterStageTrigger` (`self.GameStateRef`) (`BlueprintMapLibrary.Map_Find` (`self.StageTriggers`) (`/Game/HangUp/Blueprints/Controllers/BP_HangUpGameState.CurrentStage` (`self.GameStateRef`))))))))
  (return (`local.bResult`)))

(fn `Disconnected`
  (params (Connector :type "/Game/HangUp/Blueprints/Gameplay/InteractiveObjects/BP_SwitchConnector Object Reference"))
  (bind _correct (`self.IsConnectionCorrect` Connector))
  (if _correct
    (`/Engine/EditorBlueprintResources/StandardMacros.DecrementInt` (`self.CurrentConnectionCount`)
      (:`  `
        (`/Game/HangUp/Blueprints/Controllers/BP_HangUpGameState.DetriggerStageEvent` (`self.GameStateRef`) (`BlueprintMapLibrary.Map_Find` (`self.StageTriggers`) (`/Game/HangUp/Blueprints/Controllers/BP_HangUpGameState.CurrentStage` (`self.GameStateRef`)))))))
  (return))

(fn `InitializeBoard`
  (bind _gamestateref (`self.GameStateRef`))
  (bind _stagetrigger (make `/Game/HangUp/Blueprints/EnumStruct/StageTrigger` "NewEnumerator3" self))
  (bind _stagetrigger_2 (make `/Game/HangUp/Blueprints/EnumStruct/StageTrigger` "NewEnumerator1" self))
  (bind _stagetrigger_3 (make `/Game/HangUp/Blueprints/EnumStruct/StageTrigger` "NewEnumerator2" self))
  (`/Game/HangUp/Blueprints/Controllers/BP_HangUpGameState.RegisterStageTrigger` _gamestateref _stagetrigger_2)
  (`BlueprintMapLibrary.Map_Add` (`self.StageTriggers`) "" _stagetrigger_2)
  (`/Game/HangUp/Blueprints/Controllers/BP_HangUpGameState.RegisterStageTrigger` _gamestateref _stagetrigger_3)
  (`BlueprintMapLibrary.Map_Add` (`self.StageTriggers`) "NewEnumerator2" _stagetrigger_3)
  (`/Game/HangUp/Blueprints/Controllers/BP_HangUpGameState.RegisterStageTrigger` _gamestateref _stagetrigger)
  (`BlueprintMapLibrary.Map_Add` (`self.StageTriggers`) "NewEnumerator3" _stagetrigger))

(fn `IsConnectionCorrect`
  (params (Connector :type "/Game/HangUp/Blueprints/Gameplay/InteractiveObjects/BP_SwitchConnector Object Reference"))
  (returns (Correct :type Boolean))
  (return (`KismetArrayLibrary.Array_Contains` (`self.CorrectConnections`) Connector)))

(fn `ShufflePins`
  (locals (remainingConnectors :type "Array of /Game/HangUp/Blueprints/Gameplay/InteractiveObjects/BP_SwitchConnector Object Reference") (CorrectConnector :type "/Game/HangUp/Blueprints/Gameplay/InteractiveObjects/BP_SwitchConnector Object Reference"))
  (bind _remainingconnectors (`local.remainingConnectors`))
  (bind _returnvalue (`KismetArrayLibrary.Array_Length` _remainingconnectors))
  (bind _output (`|GetArrayItem` _remainingconnectors (`KismetMathLibrary.RandomInteger` _returnvalue)))
  (set `self.CurrentConnectionCount` 0)
  (`KismetArrayLibrary.Array_Clear` (`self.CorrectConnections`))
  (for _array_element (`self.AllSwitchConnectors`)
    (`KismetArrayLibrary.Array_Add` (`local.remainingConnectors`) _array_element))
  (for _ (range 1 (+ (`self.TotalConnectionNeeded`) 1))
    (`|ExecutionSequence`
      (:`then_0`
        (set `local.CorrectConnector` _output)
        (`KismetArrayLibrary.Array_RemoveItem` _remainingconnectors _output)
        (`KismetSystemLibrary.PrintString` (`KismetStringLibrary.Conv_IntToString` _returnvalue)))
      (:`then_1`
        (`KismetArrayLibrary.Array_Add` (`self.CorrectConnections`) (`local.CorrectConnector`))))))

(fn `UserConstructionScript`)