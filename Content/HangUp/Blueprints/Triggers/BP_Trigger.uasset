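; Generic box or capsule trigger volume that runs attached TriggerResponse components once its attached TriggerCondition components are met.
; The construction script gathers both component lists and configures bounds and label text.
; Overlap, with an actor tag check, or a disabled entry check arms it, then Tick evaluates conditions alongside a hold timer.
; After firing, an after-trigger setting can wait out the longest response, destroy the trigger or parent, or run exit-only responses.
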(event `self.ReceiveBeginPlay`
  ;[0 0 0] Comment
  (`|ExecutionSequence`
    (:`then_0`
      (if (`self.disableEntryCheck`)
        (set `self.triggered` true)))
    (:`then_1`
      (`|ExecutionSequence`
        (:`then_0`
          (for _array_element (`self.TriggerConditionsList`)
            (`/Game/HangUp/Blueprints/Triggers/TriggerCondition.OnBeginActions` _array_element)))
        (:`then_1`
          (for _array_element_2 (`self.TriggerResponsesList`)
            (`/Game/HangUp/Blueprints/Triggers/TriggerResponse.OnBeginActions` _array_element_2)))))))

(event `self.ReceiveTick`
  (params (DeltaSeconds :type "Float (single-precision)"))
  ;[0 0 0] Update
  (`|ExecutionSequence`
    (:`then_0`
      (if (`self.disableEntryCheck`)
        _))
    (:`then_1`
      (`self.CheckTriggerConditions`))))

(event `CheckTriggerConditions`
  ;[0 0 0] If triggered is true (set when an object collides with this) and the conditions haven't already been met and the responses aren't executing
  (if (and (`self.triggered`) (not (`self.responsesExecuting`)))
    (set `self.conditionMet` true) ; Default this to true
    (for _array_element (`self.TriggerConditionsList`)
      (bind _issuccess (`/Game/HangUp/Blueprints/Triggers/TriggerCondition.ExecuteActions` _array_element (`self.collidingActor`)))
      (bind _output_get (set `self.conditionMet` _issuccess))
      (if (not _output_get)
        (break)))
    (bind _conditionmet (`self.CheckConditionTimer`)) ; This function checks to make sure the conditions have been met for a certain amount of time.
    (if (and _conditionmet _output_get)
      (`self.ConditionsMet`))))

(event `ConditionsMet`
  (bind _aftertriggeraction (`self.afterTriggerAction`))
  ;[0 0 0] Conditions Met - Begin Tigger Actions and Executions
  (set `self.responsesExecuting` true)
  (set `self.waitTime` 0.0)
  (`|ExecutionSequence`
    (:`then_0`
      (if (`self.debugTriggerBox`)
        (`KismetSystemLibrary.PrintString` "Trigger Has Been Triggered")))
    (:`then_1`
      (for _array_element (`self.TriggerResponsesList`)
        (if (not (`/Game/HangUp/Blueprints/Triggers/TriggerResponse.executeOnlyOnTriggerExit` _array_element))
          (`/Game/HangUp/Blueprints/Triggers/TriggerResponse.ExecuteActions` _array_element (`self.collidingActor`)) ; Execute every response
          (bind _duration (`/Game/HangUp/Blueprints/Triggers/TriggerResponse.duration` _array_element))
          (if (> _duration (`self.waitTime`))
            (set `self.waitTime` _duration)))))
    (:`then_2`
      (if (or (`|EnumEquality` _aftertriggeraction "NewEnumerator0") (`|EnumEquality` _aftertriggeraction "NewEnumerator1") (`|EnumEquality` _aftertriggeraction "NewEnumerator2"))
        (`KismetSystemLibrary.Delay` (`self.waitTime`))
        (switch `/Game/HangUp/Blueprints/EnumStruct/AfterTriggerOptions` (`self.afterTriggerAction`)
          (:`NewEnumerator1`
            (`self.K2_DestroyActor`))
          (:`NewEnumerator2`
            (`self.K2_DestroyActor` (`self.GetParentActor`)))
          (:`NewEnumerator3`
            (set `self.conditionTimer` 0.0)
            (set `self.responsesExecuting` false)
            (if (not (`self.disableEntryCheck`))
              (set `self.triggered` false))))))))

(event `self.ReceiveActorBeginOverlap`
  (params (OtherActor :type "Actor Object Reference"))
  ;[0 0 0] Check colliding object
  (if (not (`self.disableEntryCheck`))
    (set `self.collidingActor` OtherActor)
    (if (== 0 (`KismetArrayLibrary.Array_Length` (`self.triggerableActorTags`)))
      (set `self.triggered` true :!label _label)
      (else
        (set `self.hasAnyTag` false)
        (for _array_element (`self.triggerableActorTags`)
          (if (`self.ActorHasTag` (`self.collidingActor`) _array_element)
            (set `self.hasAnyTag` true)
            (break)))
        (if (not (`self.hasAnyTag`))
          (set `self.collidingActor` null)
          (goto _label))))))

(event `self.Capsule.OnComponentEndOverlap`
  (params (OverlappedComponent :type "PrimitiveComponent Object Reference") (OtherActor :type "Actor Object Reference") (OtherComp :type "PrimitiveComponent Object Reference") (OtherBodyIndex :type Integer))
  ;[0 0 0] Comment
  (if (== OtherActor (`self.collidingActor`))
    (`|ExecutionSequence`
      (:`then_0`
        (if (`self.debugTriggerBox`)
          (`KismetSystemLibrary.PrintString` "Trigger Has Been Exited")))
      (:`then_1`
        (if (`|EnumEquality` (`self.afterTriggerAction`) "NewEnumerator4")
          (if (`self.responsesExecuting`)
            (`self.OnExitResponses`)))))
    (elif (not (`self.canWander`))
      (set `self.triggered` false) ; Else we need simply set triggered to false because the object has left the trigger box
    )))

(event `OnExitResponses`
  (for _array_element (`self.TriggerResponsesList`)
    (if (`/Game/HangUp/Blueprints/Triggers/TriggerResponse.executeOnlyOnTriggerExit` _array_element)
      (`/Game/HangUp/Blueprints/Triggers/TriggerResponse.ExecuteActions` _array_element null) ; Execute every response
      (set `self.responsesExecuting` false)
      (set `self.triggered` false)
      (set `self.conditionTimer` 0.0)
      (set `self.collidingActor` null))))

(fn `CheckConditionTimer`
  (returns (conditionMet :type Boolean))
  (if (>= (`self.conditionTimer`) (`self.conditionTime`))
    (return true)
    (else
      (set `self.conditionTimer` (+ (`GameplayStatics.GetWorldDeltaSeconds`) (`self.conditionTimer`)))
      (return false))))

(fn `UserConstructionScript`
  (bind _textrender (`self.TextRender`))
  (bind _capsule (`self.Capsule`))
  (bind _capsulehalfheight (`self.CapsuleHalfHeight`))
  (`|ExecutionSequence`
    (:`then_0`
      (set `self.TriggerConditionsList` (`self.K2_GetComponentsByClass` "/Game/HangUp/Blueprints/Triggers/TriggerCondition.TriggerCondition_C")))
    (:`then_1`
      (set `self.TriggerResponsesList` (`self.K2_GetComponentsByClass` "/Game/HangUp/Blueprints/Triggers/TriggerResponse.TriggerResponse_C")))
    (:`then_2`
      (`TextRenderComponent.K2_SetText` _textrender (`KismetTextLibrary.Conv_StringToText` (`self.DisplayedText`)))
      (`TextRenderComponent.SetTextRenderColor` _textrender (`KismetMathLibrary.Conv_LinearColorToColor` (`self.TextColor`)))
      (`BoxComponent.SetBoxExtent` (`self.Box`) (`self.boundExtent`) true)
      (`CapsuleComponent.SetCapsuleSize` _capsule (`self.CapsuleRadius`) _capsulehalfheight true)
      (`SceneComponent.K2_SetRelativeLocation` _capsule (`KismetMathLibrary.MakeVector` 0.0 0.0 (- _capsulehalfheight (`self.CapsuleRadius`))) false false))
    (:`then_3`
      (if (`self.toggleBoundType`)
        (`SceneComponent.SetHiddenInGame` (`self.Box`) true false)
        (`SceneComponent.SetHiddenInGame` (`self.Capsule`) false false)
        (`SceneComponent.SetVisibility` (`self.Box`) true false)
        (else
          (`SceneComponent.SetHiddenInGame` (`self.Capsule`) true false)
          (`SceneComponent.SetVisibility` (`self.Capsule`) true false)
          (`SceneComponent.SetHiddenInGame` (`self.Box`) false false))))))