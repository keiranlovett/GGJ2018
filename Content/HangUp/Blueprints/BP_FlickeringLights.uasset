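; BP_FlickeringLights is a light Blueprint that flickers with an electrical buzz sound.
; On BeginPlay it silences BuzzSingle and, only if CanFlicker is false, plays Timeline_LightFlicker.
; The timeline's float track, scaled by a constant, drives the intensity of LightComponent and PointLightComponent.
; Its Toggle event track runs a FlipFlop that restarts the buzz on alternate triggers and writes CanFlicker, which is checked only at BeginPlay.
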(event `self.ReceiveBeginPlay`
  (`AudioComponent.Stop` (`self.buzzSingle`))
  (if (not (`self.canFlicker`))
    (bind (_direction _newtrack_0) (`Timeline|Timeline_LightFlicker`)
      (:`Update`
        (`LightComponent.SetIntensity` (`self.LightComponent`) (* _newtrack_0 300.0))
        (`LightComponent.SetIntensity` (`self.PointLightComponent`) (* _newtrack_0 300.0)))
      (:`TriggerToggle`
        (bind _isa (`/Engine/EditorBlueprintResources/StandardMacros.FlipFlop`)
          (:`A`
            (`AudioComponent.Play` (`self.buzzSingle`) 0.0))
          (:`B`
            _))
        (set `self.canFlicker` _isa)))))

(fn `UserConstructionScript`)